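; BP_Ghost is a wandering NPC that bursts into leaves when struck by a projectile.
; After a short startup delay it loops AIMoveTo to random reachable nearby points, pausing between moves and retrying quickly on failure.
; A hit from a "Projectile"-tagged actor spawns Niagara leaves driven by scaled projectile velocity, hides the mesh, disables capsule collision, then destroys the ghost after a delay.
; Tick turns the health bar widget toward the camera.
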(event `self.ReceiveBeginPlay`
  (`KismetSystemLibrary.Delay` 1.0)
  (`self.MoveNPC`))

(event `MoveNPC`
  (`|AIMoveTo` self (`NavigationSystemV1.K2_GetRandomReachablePointInRadius` (`self.K2_GetActorLocation`) 1000.0 null null) null
    (:`OnSuccess`
      (`KismetSystemLibrary.Delay` 4.0)
      (`self.MoveNPC`))
    (:`OnFail`
      (`KismetSystemLibrary.Delay` 0.2)
      (`self.MoveNPC`))))

(event `self.ReceiveHit`
  (params (MyComp :type "PrimitiveComponent Object Reference") (Other :type "Actor Object Reference") (OtherComp :type "PrimitiveComponent Object Reference") (bSelfMoved :type Boolean) (HitLocation :type "Vector Structure") (HitNormal :type "Vector Structure") (NormalImpulse :type "Vector Structure") (Hit :type "HitResult Structure (by ref)"))
  (if (`self.ActorHasTag` Other "Projectile")
    (bind _returnvalue (`NiagaraFunctionLibrary.SpawnSystemAttached` "/Game/Niagara/NS_Leaf.NS_Leaf" MyComp "None" (0.0 0.0 0.0) (struct) "KeepRelativeOffset"))
    (`NiagaraComponent.SetVariableVec3` _returnvalue "WindSpeed" (* (`self.GetVelocity` Other) (0.2 0.2 0.2)))
    (`SceneComponent.SetVisibility` (`self.Mesh`) false false)
    (`PrimitiveComponent.SetCollisionEnabled` (`self.Capsule`) "NoCollision")
    (`PrimitiveComponent.SetCollisionEnabled` (`self.CapsuleComponent`) "NoCollision")
    (`KismetSystemLibrary.Delay` 4.0)
    (`self.K2_DestroyActor`)))

(event `self.ReceiveTick`
  (params (DeltaSeconds :type "Float (single-precision)"))
  (bind _widget_healthbar (`self.Widget_HealthBar`))
  (`SceneComponent.K2_SetWorldRotation` _widget_healthbar (`KismetMathLibrary.FindLookAtRotation` (`SceneComponent.K2_GetComponentLocation` _widget_healthbar) (`SceneComponent.K2_GetComponentLocation` (`PlayerCameraManager.TransformComponent` (`GameplayStatics.GetPlayerCameraManager` 0)))) false false))

(fn `UserConstructionScript`)